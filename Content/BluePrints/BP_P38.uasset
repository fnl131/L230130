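; BP_P38 is a player-controlled P-38 plane pawn that constantly flies forward.
; Tick applies forward movement input and spins the Right and LEFT propeller components through NewFunction at ProfellaRotationSpeed.
; Pitch and Roll axes feed controller rotation input, and Fire spawns a BP_Locket at the Arrow component's transform.
; Direct actor rotation and offset nodes using RotationSpeed and MoveSpeed are left unconnected.
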(event EventBeginPlay)

(event Collision|EventActorBeginOverlap
  (params (OtherActor :type Actor%20Object%20Reference)))

(event EventTick
  (params (DeltaSeconds :type Float%20%28single-precision%29))
  (CallFunction|NewFunction (Variables|Default|GetRight))
  (CallFunction|NewFunction (Variables|Default|GetLEFT))
  (Pawn|Input|AddMovementInput (Transformation|GetActorForwardVector) 1.0 false))

(event Input|ActionEvents|InputActionFire
  (params (Key :type Key%20Structure :default "None"))
  (:Pressed
    (Game|SpawnActorfromClass "/Game/BluePrints/BP_Locket.BP_Locket_C" (Transformation|GetWorldTransform (Variables|Default|GetArrow)) "AdjustIfPossibleButDontSpawnIfColliding" 0 0)))

(event Input|AxisEvents|InputAxisPitch
  (params (AxisValue :type Float%20%28single-precision%29))
  (Pawn|Input|AddControllerPitchInput AxisValue))

(event Input|AxisEvents|InputAxisRoll
  (params (AxisValue :type Float%20%28single-precision%29))
  (Pawn|Input|AddControllerRollInput AxisValue))

(fn ConstructionScript)

(fn NewFunction
  (params (self2 :type Scene%20Component%20Object%20Reference))
  (Transformation|AddLocalRotation self2 (Math|Rotator|MakeRotator (* (Utilities|Time|GetWorldDeltaSeconds) (Variables|Default|GetProfella%20Rotation%20Speed)) 0.0 0.0) false false))