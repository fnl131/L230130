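; BP_Pawn is a player-controlled twin-propeller aircraft that flies forward constantly and fires rockets.
; BeginPlay adds the IAC_Inputs Enhanced Input mapping context, and Tick applies forward movement input while spinning the Left and Right propellers, scaled by delta time.
; The IA_PitchANdRoll action feeds controller pitch and roll for steering, and the Fire action spawns BP_Rocket at the Arrow component's transform.
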(event Input|EnhancedActionEvents|EnhancedInputActionIA_PitchANdRoll
  (params (ActionValue :type Vector%202D%20Structure) (ElapsedSeconds :type Float%20%28double-precision%29) (TriggeredSeconds :type Float%20%28double-precision%29) (InputAction :type Input%20Action%20Object%20Reference :default "/Game/BluePrints/inputs/IA_PitchANdRoll.IA_PitchANdRoll"))
  (:Triggered
    (Pawn|Input|AddControllerPitchInput (.y ActionValue))
    (Pawn|Input|AddControllerRollInput (.x ActionValue))))

(event EventBeginPlay
  (bind _returnvalue (Game|GetPlayerController 0))
  (Utilities|IsValid _returnvalue
    (:Is%20Valid
      (Input|AddMappingContext (PlayerController|LocalPlayerSubsystems|GetEnhancedInputLocalPlayerSubsystem _returnvalue) "/Game/BluePrints/inputs/IAC_Inputs.IAC_Inputs" 0 "(bIgnoreAllPressedKeysUntilRelease=True,bForceImmediately=False)"))))

(event EventTick
  (params (DeltaSeconds :type Float%20%28single-precision%29))
  ;[1 1 1] 무브먼트 이동
  (Pawn|Input|AddMovementInput (Transformation|GetActorForwardVector) 1.0 false)
  ;[1 1 1] 왼쪽 프로펠러 회전
  (Transformation|AddLocalRotation (Variables|Default|GetLeft) (* (Variables|속력|GetPropellerRotationSpeed) (Utilities|Time|GetWorldDeltaSeconds)) false false)
  ;[1 1 1] 오른쪽 프로펠러 회전
  (Transformation|AddLocalRotation (Variables|Default|GetRight) (* (Variables|속력|GetPropellerRotationSpeed) (Utilities|Time|GetWorldDeltaSeconds)) false false))

(event Input|ActionEvents|InputActionFire
  (params (Key :type Key%20Structure :default "None"))
  ;[1 1 1] 미사일 발사
  (:Pressed
    (Game|SpawnActorfromClass "/Game/BluePrints/BP_Rocket.BP_Rocket_C" (Transformation|GetWorldTransform (Variables|Default|GetArrow)) "Undefined" 0 0)))

(fn ConstructionScript)